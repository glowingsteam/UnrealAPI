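; Test pawn for exercising HTTP calls from the game to a local choices web API.
; On BeginPlay it binds a completion callback on the web communication target that prints the status code and each returned data element.
; Pressing 3 builds and sends a POST with a hardcoded JSON body and custom headers to a localhost endpoint.
; An unconnected HTTPS variant of the same request is left in the graph.
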(event `self.ReceiveBeginPlay`
  (add `WebCommunicationBPLibrary.onhttpRequestCompleteDelegate` (`WebCommunicationBPLibrary.getWebCommunicationTarget`) (delegate `HTTPRequestComplete`)))

(event `HTTPRequestComplete`
  (params (data :type "Array of String (by ref)") (statusCode :type Integer) (byteData :type "Array of Byte (by ref)") (requestID :type String))
  (`KismetSystemLibrary.PrintString` (`KismetStringLibrary.Conv_IntToString` statusCode))
  (for _array_element data
    (`KismetSystemLibrary.PrintString` _array_element)))

(event `Key|Three`
  (params (Key :type "Key Structure"))
  (:`Pressed`
    (bind _httprequests (`WebCommunicationBPLibrary.CreateHttpRequestIndividual` :`url` "http://localhost:50793/api/choices" :`header` (`|MakeMap` "Content-Type" "application/json" "User-Agent" "DefusalGame/0.1" "Accept" "*/*" "Accept-Encoding" "gzip, deflate, br" "Connection" "keep-alive") :`verb` "POST" :`content` "{ \n	\"firstName\": \"John\", \n	\"number\": 5 \n}"))
    (`WebCommunicationBPLibrary.executeHttpRequests` _httprequests)))

(fn `UserConstructionScript`)